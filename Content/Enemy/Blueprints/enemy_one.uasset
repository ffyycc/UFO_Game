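; Enemy actor that fires Magic_ball projectiles in repeating volleys and can be killed by the player ufo's attack balls.
; A BeginPlay loop alternates timed QuickShootFront bursts with idle pauses, launching each ball along fixed world X.
; An Eyesight overlap toggles the HP bar widget, which receives a reference to this enemy.
; Attack-ball overlaps subtract PlayerDamage; at zero HP a sequence destroys the actor and awards the player a coin.
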(event OnComponentBeginOverlap(eyesight)
  (params (OverlappedComponent :type Primitive%20Component%20Object%20Reference) (OtherActor :type Actor%20Object%20Reference) (OtherComp :type Primitive%20Component%20Object%20Reference) (OtherBodyIndex :type Integer) (bFromSweep :type Boolean) (SweepResult :type Hit%20Result%20Structure%20%28by%20ref%29))
  ;[1 1 1] hp bar visualbility
  (Utilities|Casting|CastToufo OtherActor)
  (Rendering|SetVisibility (Variables|Default|Getenemy_hp) true false))

(event OnComponentEndOverlap(eyesight)
  (params (OverlappedComponent :type Primitive%20Component%20Object%20Reference) (OtherActor :type Actor%20Object%20Reference) (OtherComp :type Primitive%20Component%20Object%20Reference) (OtherBodyIndex :type Integer))
  ;[1 1 1] hp bar visualbility
  (Utilities|Casting|CastToufo OtherActor)
  (Rendering|SetVisibility (Variables|Default|Getenemy_hp) false false))

(event OnComponentBeginOverlap(enemycollision)
  (params (OverlappedComponent :type Primitive%20Component%20Object%20Reference) (OtherActor :type Actor%20Object%20Reference) (OtherComp :type Primitive%20Component%20Object%20Reference) (OtherBodyIndex :type Integer) (bFromSweep :type Boolean) (SweepResult :type Hit%20Result%20Structure%20%28by%20ref%29))
  ;[1 1 1] take damge from player
  (Utilities|Casting|CastToattack_ball_player OtherActor)
  (CallFunction|TakeDamage)
  (if (and (<= (Variables|Default|Getcur_hp) 0) (not (Variables|Default|Getdeath_anime)))
    (Utilities|FlowControl|Sequence
      (:then_0
        (Actor|DestroyActor))
      (:then_1
        (bind _asufo (Utilities|Casting|CastToufo (Game|Player|GetPlayerPawn 0)))
        (Default|AddCoin _asufo)
        (Actor|DestroyActor)))))

(event EventBeginPlay
  ;[1 1 1] cast to hp
  (bind _asenemy_one_hp (Utilities|Casting|CastToenemy_one_hp (UserInterface|GetUserWidgetObject (Variables|Default|Getenemy_hp))))
  (Variables|/Game/Enemy/Blueprints/enemy_one_hp.enemy_one_hp_C|Setenemy_one_ref _asenemy_one_hp self)
  (Rendering|SetVisibility (Variables|Default|Getenemy_hp) false false)
  ;[1 1 1] make projectile
  (if (not (Variables|Default|Getdeath_anime)) :!label _label
    (if (> (Variables|Default|GetIndex) 0)
      (Variables|Default|SetIndex (- (Variables|Default|GetIndex) 1))
      (Utilities|FlowControl|Delay 0.3)
      (CallFunction|QuickShootFront)
      (goto _label)
      (elif (not (Variables|Default|Getdeath_anime))
        (Components|Animation|PlayAnimation (Variables|Character|GetMesh) "/Game/FourEvilDragonsPBR/Animations/DragonTheNightmare/Idle01Anim.Idle01Anim" false)
        (Utilities|FlowControl|Delay 1.0)
        (Variables|Default|SetIndex 5)
        (goto _label)))))

(fn ConstructionScript)

(fn QuickShootFront
  (bind _magicballfront (Variables|Default|GetMagicBallFront))
  (if (Variables|Default|Getdeath_anime)
    _
    (else
      _))
  (Components|Animation|PlayAnimation (Variables|Character|GetMesh) "/Game/FourEvilDragonsPBR/Animations/DragonTheNightmare/AttackMouthAnim.AttackMouthAnim" false)
  (bind _returnvalue (Game|SpawnActorfromClass "/Game/Enemy/Blueprints/magic_ball.magic_ball_C" (Math|Transform|MakeTransform (Transformation|GetWorldLocation _magicballfront) (Transformation|GetWorldRotation _magicballfront) "1,1,1") "Undefined" 0 0))
  (Class|PrimitiveComponent|SetAllPhysicsLinearVelocity (Variables|/Game/Enemy/Blueprints/magic_ball.magic_ball_C|GetSphere _returnvalue) "100.000000, 0, 0" false))

(fn TakeDamage
  (Variables|Default|Setcur_hp (- (Variables|Default|Getcur_hp) (Variables|Default|Getplayer_damage))))