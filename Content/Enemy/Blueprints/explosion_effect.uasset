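; Enemy explosion effect actor that damages the ufo and then removes itself.
; Overlap with its Explosion_range component casts the other actor to ufo and subtracts a fixed amount from its Health.
; Any actor overlap destroys the PExplosion component, then the actor after a short delay.
; A P_Explosion overlap with anything but the player pawn also triggers delayed self-destruction.
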(event OnComponentBeginOverlap(explosion_range)
  (params (OverlappedComponent :type Primitive%20Component%20Object%20Reference) (OtherActor :type Actor%20Object%20Reference) (OtherComp :type Primitive%20Component%20Object%20Reference) (OtherBodyIndex :type Integer) (bFromSweep :type Boolean) (SweepResult :type Hit%20Result%20Structure%20%28by%20ref%29))
  (bind _asufo (Utilities|Casting|CastToufo OtherActor))
  (Variables|/Game/D_ufo/ufo.ufo_C|SetHealth _asufo (- (Variables|/Game/D_ufo/ufo.ufo_C|GetHealth _asufo) 0.3)))

(event OnComponentBeginOverlap(P_Explosion)
  (params (OverlappedComponent :type Primitive%20Component%20Object%20Reference) (OtherActor :type Actor%20Object%20Reference) (OtherComp :type Primitive%20Component%20Object%20Reference) (OtherBodyIndex :type Integer) (bFromSweep :type Boolean) (SweepResult :type Hit%20Result%20Structure%20%28by%20ref%29))
  (if (not (== OtherActor (Game|Player|GetPlayerPawn 0)))
    (Utilities|FlowControl|Delay 0.5)
    (Actor|DestroyActor)))

(event Collision|EventActorBeginOverlap
  (params (OtherActor :type Actor%20Object%20Reference))
  (Components|DestroyComponent (Variables|Default|GetP_Explosion))
  (Utilities|FlowControl|Delay 0.1)
  (Actor|DestroyActor))

(event EventTick
  (params (DeltaSeconds :type Float%20%28single-precision%29)))

(fn ConstructionScript)