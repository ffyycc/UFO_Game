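; Kraken-animated enemy that sweeps Magic_ball projectiles across five forward spawn points, left to right, in a delayed loop until death.
; An Eyesight overlap toggles its HP bar widget when the ufo enters or leaves.
; Player attack balls reduce HP; at zero it plays death and awards a coin, but immediate destruction preempts the six-second delay.
; QuickShootFront and ShootThreeDirections are defined but not called here.
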(event OnComponentBeginOverlap(eyesight)
  (params (OverlappedComponent :type Primitive%20Component%20Object%20Reference) (OtherActor :type Actor%20Object%20Reference) (OtherComp :type Primitive%20Component%20Object%20Reference) (OtherBodyIndex :type Integer) (bFromSweep :type Boolean) (SweepResult :type Hit%20Result%20Structure%20%28by%20ref%29))
  ;[1 1 1] hp bar visualbility
  (Utilities|Casting|CastToufo OtherActor)
  (Rendering|SetVisibility (Variables|Default|Gethp_bar) true false))

(event OnComponentEndOverlap(eyesight)
  (params (OverlappedComponent :type Primitive%20Component%20Object%20Reference) (OtherActor :type Actor%20Object%20Reference) (OtherComp :type Primitive%20Component%20Object%20Reference) (OtherBodyIndex :type Integer))
  ;[1 1 1] hp bar visualbility
  (Utilities|Casting|CastToufo OtherActor)
  (Rendering|SetVisibility (Variables|Default|Gethp_bar) false false))

(event OnComponentBeginOverlap(enemycollision)
  (params (OverlappedComponent :type Primitive%20Component%20Object%20Reference) (OtherActor :type Actor%20Object%20Reference) (OtherComp :type Primitive%20Component%20Object%20Reference) (OtherBodyIndex :type Integer) (bFromSweep :type Boolean) (SweepResult :type Hit%20Result%20Structure%20%28by%20ref%29))
  ;[1 1 1] enemy hit
  (Utilities|Casting|CastToattack_ball_player OtherActor)
  (CallFunction|TakeDamage)
  (if (and (<= (Variables|Default|Getcur_hp) 0) (not (Variables|Default|GetDeathAnime)))
    (Utilities|FlowControl|Sequence
      (:then_0
        (Variables|Default|SetDeathAnime true)
        (Components|Animation|PlayAnimation (Variables|Character|GetMesh) "/Game/EnemyMaterialAndParticle/KRAKEN_death.KRAKEN_death" false)
        (Utilities|FlowControl|Delay 6.0)
        (Actor|DestroyActor))
      (:then_1
        (bind _asufo (Utilities|Casting|CastToufo (Game|Player|GetPlayerPawn 0)))
        (Default|AddCoin _asufo)
        (Actor|DestroyActor)))))

(event EventBeginPlay
  (bind _delay_time (Variables|Default|GetDelay_time))
  ;[1 1 1] initialize hp bar
  (bind _asenemy_four_hp (Utilities|Casting|CastToenemy_four_hp (UserInterface|GetWidget (Variables|Default|Gethp_bar))))
  (Variables|/Game/Enemy/Blueprints/enemy_four_hp.enemy_four_hp_C|Setenemy_four_ref _asenemy_four_hp self)
  (Rendering|SetVisibility (Variables|Default|Gethp_bar) false false)
  ;[1 1 1] make projectile
  (if (not (Variables|Default|GetDeathAnime)) :!label _label
    (Components|Animation|PlayAnimation (Variables|Character|GetMesh) "/Game/Kraken/Animations/KRAKEN_sweepAttack.KRAKEN_sweepAttack" false)
    (Utilities|FlowControl|Delay (Variables|Default|GetDelay_time))
    (CallFunction|ShootLeftFront)
    (Utilities|FlowControl|Delay _delay_time)
    (CallFunction|ShootFrontLeft)
    (Utilities|FlowControl|Delay _delay_time)
    (CallFunction|ShootFront)
    (Utilities|FlowControl|Delay _delay_time)
    (CallFunction|ShootFrontRight)
    (Utilities|FlowControl|Delay _delay_time)
    (CallFunction|ShootRightFront)
    (Utilities|FlowControl|Delay (Variables|Default|GetAttack_gap))
    (goto _label)))

(fn ConstructionScript)

(fn QuickShootFront
  (bind _magicballfront (Variables|Default|GetMagicBallFront))
  (bind _returnvalue (Game|SpawnActorfromClass "/Game/Enemy/Blueprints/magic_ball.magic_ball_C" (Math|Transform|MakeTransform (Transformation|GetWorldLocation _magicballfront) (Transformation|GetWorldRotation _magicballfront) "1,1,1") "Undefined" 0 0))
  (Class|PrimitiveComponent|SetAllPhysicsLinearVelocity (Variables|/Game/Enemy/Blueprints/magic_ball.magic_ball_C|GetSphere _returnvalue) "100.000000, 0, 0" false))

(fn ShootThreeDirections
  (bind _magicballfront (Variables|Default|GetMagicBallFront))
  (bind _returnvalue (Game|SpawnActorfromClass "/Game/Enemy/Blueprints/magic_ball.magic_ball_C" (Math|Transform|MakeTransform (Transformation|GetWorldLocation _magicballfront) (Transformation|GetWorldRotation _magicballfront) "1,1,1") "Undefined" 0 0))
  (Class|PrimitiveComponent|SetAllPhysicsLinearVelocity (Variables|/Game/Enemy/Blueprints/magic_ball.magic_ball_C|GetSphere _returnvalue) "100.000000, 0, 0" false)
  (Game|SpawnActorfromClass "/Game/Enemy/Blueprints/magic_ball.magic_ball_C" (Transformation|GetWorldTransform (Variables|Default|GetMagicBallLeftFront)) "Undefined" 0 0)
  (Game|SpawnActorfromClass "/Game/Enemy/Blueprints/magic_ball.magic_ball_C" (Transformation|GetWorldTransform (Variables|Default|GetMagicBallRightFront)) "Undefined" 0 0))

(fn ShootLeftFront
  (Game|SpawnActorfromClass "/Game/Enemy/Blueprints/magic_ball.magic_ball_C" (Transformation|GetWorldTransform (Variables|Default|GetMagicBallLeftFront)) "Undefined" 0 0))

(fn ShootFrontLeft
  (Game|SpawnActorfromClass "/Game/Enemy/Blueprints/magic_ball.magic_ball_C" (Transformation|GetWorldTransform (Variables|Default|GetMagicBallFrontLeft)) "Undefined" 0 0))

(fn ShootFront
  (Game|SpawnActorfromClass "/Game/Enemy/Blueprints/magic_ball.magic_ball_C" (Transformation|GetWorldTransform (Variables|Default|GetMagicBallFront)) "Undefined" 0 0))

(fn ShootFrontRight
  (Game|SpawnActorfromClass "/Game/Enemy/Blueprints/magic_ball.magic_ball_C" (Transformation|GetWorldTransform (Variables|Default|GetMagicBallFrontRight)) "Undefined" 0 0))

(fn ShootRightFront
  (Game|SpawnActorfromClass "/Game/Enemy/Blueprints/magic_ball.magic_ball_C" (Transformation|GetWorldTransform (Variables|Default|GetMagicBallRightFront)) "Undefined" 0 0))

(fn TakeDamage
  (Variables|Default|Setcur_hp (- (Variables|Default|Getcur_hp) (Variables|Default|Getplayer_damage))))