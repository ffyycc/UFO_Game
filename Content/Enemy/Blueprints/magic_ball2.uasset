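; Enemy magic ball actor that damages a ufo on contact and expires after a set lifetime.
; Any overlap on its Sphere spawns an ice explosion with no location wired in and destroys the ball, then subtracts a fixed amount of Health if the other actor is a ufo.
; BeginPlay waits TimeExist, then spawns the same explosion at the Sphere's transform and destroys the actor.
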(event OnComponentBeginOverlap(Sphere)
  (params (OverlappedComponent :type Primitive%20Component%20Object%20Reference) (OtherActor :type Actor%20Object%20Reference) (OtherComp :type Primitive%20Component%20Object%20Reference) (OtherBodyIndex :type Integer) (bFromSweep :type Boolean) (SweepResult :type Hit%20Result%20Structure%20%28by%20ref%29))
  (Effects|SpawnEmitteratLocation "/Game/EnemyMaterialAndParticle/P_ProjectileLob_Explo_Ice_02.P_ProjectileLob_Explo_Ice_02" "0, 0, 0")
  (Actor|DestroyActor)
  (bind _asufo (Utilities|Casting|CastToufo OtherActor))
  (Variables|/Game/D_ufo/ufo.ufo_C|SetHealth _asufo (- (Variables|/Game/D_ufo/ufo.ufo_C|GetHealth _asufo) 0.2)))

(event EventBeginPlay
  (bind _sphere (Variables|Default|GetSphere))
  (Utilities|FlowControl|Delay (Variables|Default|Gettime_exist))
  (Effects|SpawnEmitteratLocation "/Game/EnemyMaterialAndParticle/P_ProjectileLob_Explo_Ice_02.P_ProjectileLob_Explo_Ice_02" (Transformation|GetWorldLocation _sphere) (Transformation|GetWorldRotation _sphere))
  (Actor|DestroyActor))

(fn ConstructionScript)