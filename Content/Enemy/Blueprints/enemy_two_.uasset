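; Second enemy type that fires a three-way magic ball volley every second from BeginPlay, whether or not the player is near.
; Its HP widget receives a self reference and shows only while the ufo player overlaps the Eyesight volume.
; Player attack balls hitting EnemyCollision subtract PlayerDamage from CurHp; at zero the enemy is destroyed and awards the ufo a coin.
; QuickShootFront, an animated single front shot, is defined but not called here.
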(event OnComponentBeginOverlap(eyesight)
  (params (OverlappedComponent :type Primitive%20Component%20Object%20Reference) (OtherActor :type Actor%20Object%20Reference) (OtherComp :type Primitive%20Component%20Object%20Reference) (OtherBodyIndex :type Integer) (bFromSweep :type Boolean) (SweepResult :type Hit%20Result%20Structure%20%28by%20ref%29))
  ;[1 1 1] hp bar visualbility
  (Utilities|Casting|CastToufo OtherActor)
  (Rendering|SetVisibility (Variables|Default|Getenemy_hp) true false))

(event OnComponentEndOverlap(eyesight)
  (params (OverlappedComponent :type Primitive%20Component%20Object%20Reference) (OtherActor :type Actor%20Object%20Reference) (OtherComp :type Primitive%20Component%20Object%20Reference) (OtherBodyIndex :type Integer))
  ;[1 1 1] hp bar visualbility
  (Utilities|Casting|CastToufo OtherActor)
  (Rendering|SetVisibility (Variables|Default|Getenemy_hp) false false))

(event OnComponentBeginOverlap(enemycollision)
  (params (OverlappedComponent :type Primitive%20Component%20Object%20Reference) (OtherActor :type Actor%20Object%20Reference) (OtherComp :type Primitive%20Component%20Object%20Reference) (OtherBodyIndex :type Integer) (bFromSweep :type Boolean) (SweepResult :type Hit%20Result%20Structure%20%28by%20ref%29))
  ;[1 1 1] take damge from player
  (Utilities|Casting|CastToattack_ball_player OtherActor)
  (CallFunction|TakeDamage)
  (if (<= (Variables|Default|Getcur_hp) 0)
    (Actor|DestroyActor)
    (bind _asufo (Utilities|Casting|CastToufo (Game|Player|GetPlayerPawn 0)))
    (Default|AddCoin _asufo)
    (Actor|DestroyActor)))

(event EventBeginPlay
  ;[1 1 1] cast to hp
  (bind _asenemy_two_hp_ (Utilities|Casting|CastToenemy_two_hp_ (UserInterface|GetUserWidgetObject (Variables|Default|Getenemy_hp))))
  (Variables|/Game/Enemy/Blueprints/enemy_two_hp_.enemy_two_hp__C|Setenemy_two_ref _asenemy_two_hp_ self)
  (Rendering|SetVisibility (Variables|Default|Getenemy_hp) false false)
  ;[1 1 1] loop
  (Utilities|FlowControl|Delay 1.0 :!label _label)
  (CallFunction|ShootThreeDirection)
  (goto _label))

(fn ConstructionScript)

(fn QuickShootFront
  (bind _magicballfront (Variables|Default|GetMagicBallFront))
  (if (Variables|Default|Getdeath_anime)
    _
    (else
      _))
  (Components|Animation|PlayAnimation (Variables|Character|GetMesh) "/Game/FourEvilDragonsPBR/Animations/DragonTheNightmare/AttackMouthAnim.AttackMouthAnim" false)
  (bind _returnvalue (Game|SpawnActorfromClass "/Game/Enemy/Blueprints/magic_ball.magic_ball_C" (Math|Transform|MakeTransform (Transformation|GetWorldLocation _magicballfront) (Transformation|GetWorldRotation _magicballfront) "1,1,1") "Undefined" 0 0))
  (Class|PrimitiveComponent|SetAllPhysicsLinearVelocity (Variables|/Game/Enemy/Blueprints/magic_ball.magic_ball_C|GetSphere _returnvalue) "100.000000, 0, 0" false))

(fn TakeDamage
  (Variables|Default|Setcur_hp (- (Variables|Default|Getcur_hp) (Variables|Default|Getplayer_damage))))

(fn ShootThreeDirection
  (bind _magicballfront (Variables|Default|GetMagicBallFront))
  (bind _returnvalue (Game|SpawnActorfromClass "/Game/Enemy/Blueprints/magic_ball.magic_ball_C" (Math|Transform|MakeTransform (Transformation|GetWorldLocation _magicballfront) (Transformation|GetWorldRotation _magicballfront) "1,1,1") "Undefined" 0 0))
  (Class|PrimitiveComponent|SetAllPhysicsLinearVelocity (Variables|/Game/Enemy/Blueprints/magic_ball.magic_ball_C|GetSphere _returnvalue) "100.000000, 0, 0" false)
  (Game|SpawnActorfromClass "/Game/Enemy/Blueprints/magic_ball.magic_ball_C" (Transformation|GetWorldTransform (Variables|Default|GetMagicBallLeftFront)) "Undefined" 0 0)
  (Game|SpawnActorfromClass "/Game/Enemy/Blueprints/magic_ball.magic_ball_C" (Transformation|GetWorldTransform (Variables|Default|GetMagicBallRightFront)) "Undefined" 0 0))