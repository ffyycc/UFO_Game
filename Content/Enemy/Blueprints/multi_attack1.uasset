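; Timed enemy multi-attack actor that damages ufo actors through a set of overlap components.
; Each of the fifteen D components has its own identical begin-overlap handler that casts the other actor to ufo and subtracts a small fixed amount from its Health.
; On BeginPlay it waits TimeExist, spawns an ice explosion emitter at the MutiAttack2 component's transform, then destroys itself.
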(event OnComponentBeginOverlap(d2)
  (params (OverlappedComponent :type Primitive%20Component%20Object%20Reference) (OtherActor :type Actor%20Object%20Reference) (OtherComp :type Primitive%20Component%20Object%20Reference) (OtherBodyIndex :type Integer) (bFromSweep :type Boolean) (SweepResult :type Hit%20Result%20Structure%20%28by%20ref%29))
  (bind _asufo (Utilities|Casting|CastToufo OtherActor))
  (Variables|/Game/D_ufo/ufo.ufo_C|SetHealth _asufo (- (Variables|/Game/D_ufo/ufo.ufo_C|GetHealth _asufo) 0.1)))

(event OnComponentBeginOverlap(d3)
  (params (OverlappedComponent :type Primitive%20Component%20Object%20Reference) (OtherActor :type Actor%20Object%20Reference) (OtherComp :type Primitive%20Component%20Object%20Reference) (OtherBodyIndex :type Integer) (bFromSweep :type Boolean) (SweepResult :type Hit%20Result%20Structure%20%28by%20ref%29))
  (bind _asufo (Utilities|Casting|CastToufo OtherActor))
  (Variables|/Game/D_ufo/ufo.ufo_C|SetHealth _asufo (- (Variables|/Game/D_ufo/ufo.ufo_C|GetHealth _asufo) 0.1)))

(event OnComponentBeginOverlap(d4)
  (params (OverlappedComponent :type Primitive%20Component%20Object%20Reference) (OtherActor :type Actor%20Object%20Reference) (OtherComp :type Primitive%20Component%20Object%20Reference) (OtherBodyIndex :type Integer) (bFromSweep :type Boolean) (SweepResult :type Hit%20Result%20Structure%20%28by%20ref%29))
  (bind _asufo (Utilities|Casting|CastToufo OtherActor))
  (Variables|/Game/D_ufo/ufo.ufo_C|SetHealth _asufo (- (Variables|/Game/D_ufo/ufo.ufo_C|GetHealth _asufo) 0.1)))

(event OnComponentBeginOverlap(d5)
  (params (OverlappedComponent :type Primitive%20Component%20Object%20Reference) (OtherActor :type Actor%20Object%20Reference) (OtherComp :type Primitive%20Component%20Object%20Reference) (OtherBodyIndex :type Integer) (bFromSweep :type Boolean) (SweepResult :type Hit%20Result%20Structure%20%28by%20ref%29))
  (bind _asufo (Utilities|Casting|CastToufo OtherActor))
  (Variables|/Game/D_ufo/ufo.ufo_C|SetHealth _asufo (- (Variables|/Game/D_ufo/ufo.ufo_C|GetHealth _asufo) 0.1)))

(event OnComponentBeginOverlap(d6)
  (params (OverlappedComponent :type Primitive%20Component%20Object%20Reference) (OtherActor :type Actor%20Object%20Reference) (OtherComp :type Primitive%20Component%20Object%20Reference) (OtherBodyIndex :type Integer) (bFromSweep :type Boolean) (SweepResult :type Hit%20Result%20Structure%20%28by%20ref%29))
  (bind _asufo (Utilities|Casting|CastToufo OtherActor))
  (Variables|/Game/D_ufo/ufo.ufo_C|SetHealth _asufo (- (Variables|/Game/D_ufo/ufo.ufo_C|GetHealth _asufo) 0.1)))

(event OnComponentBeginOverlap(d15)
  (params (OverlappedComponent :type Primitive%20Component%20Object%20Reference) (OtherActor :type Actor%20Object%20Reference) (OtherComp :type Primitive%20Component%20Object%20Reference) (OtherBodyIndex :type Integer) (bFromSweep :type Boolean) (SweepResult :type Hit%20Result%20Structure%20%28by%20ref%29))
  (bind _asufo (Utilities|Casting|CastToufo OtherActor))
  (Variables|/Game/D_ufo/ufo.ufo_C|SetHealth _asufo (- (Variables|/Game/D_ufo/ufo.ufo_C|GetHealth _asufo) 0.1)))

(event OnComponentBeginOverlap(d7)
  (params (OverlappedComponent :type Primitive%20Component%20Object%20Reference) (OtherActor :type Actor%20Object%20Reference) (OtherComp :type Primitive%20Component%20Object%20Reference) (OtherBodyIndex :type Integer) (bFromSweep :type Boolean) (SweepResult :type Hit%20Result%20Structure%20%28by%20ref%29))
  (bind _asufo (Utilities|Casting|CastToufo OtherActor))
  (Variables|/Game/D_ufo/ufo.ufo_C|SetHealth _asufo (- (Variables|/Game/D_ufo/ufo.ufo_C|GetHealth _asufo) 0.1)))

(event OnComponentBeginOverlap(d8)
  (params (OverlappedComponent :type Primitive%20Component%20Object%20Reference) (OtherActor :type Actor%20Object%20Reference) (OtherComp :type Primitive%20Component%20Object%20Reference) (OtherBodyIndex :type Integer) (bFromSweep :type Boolean) (SweepResult :type Hit%20Result%20Structure%20%28by%20ref%29))
  (bind _asufo (Utilities|Casting|CastToufo OtherActor))
  (Variables|/Game/D_ufo/ufo.ufo_C|SetHealth _asufo (- (Variables|/Game/D_ufo/ufo.ufo_C|GetHealth _asufo) 0.1)))

(event OnComponentBeginOverlap(d9)
  (params (OverlappedComponent :type Primitive%20Component%20Object%20Reference) (OtherActor :type Actor%20Object%20Reference) (OtherComp :type Primitive%20Component%20Object%20Reference) (OtherBodyIndex :type Integer) (bFromSweep :type Boolean) (SweepResult :type Hit%20Result%20Structure%20%28by%20ref%29))
  (bind _asufo (Utilities|Casting|CastToufo OtherActor))
  (Variables|/Game/D_ufo/ufo.ufo_C|SetHealth _asufo (- (Variables|/Game/D_ufo/ufo.ufo_C|GetHealth _asufo) 0.1)))

(event OnComponentBeginOverlap(d10)
  (params (OverlappedComponent :type Primitive%20Component%20Object%20Reference) (OtherActor :type Actor%20Object%20Reference) (OtherComp :type Primitive%20Component%20Object%20Reference) (OtherBodyIndex :type Integer) (bFromSweep :type Boolean) (SweepResult :type Hit%20Result%20Structure%20%28by%20ref%29))
  (bind _asufo (Utilities|Casting|CastToufo OtherActor))
  (Variables|/Game/D_ufo/ufo.ufo_C|SetHealth _asufo (- (Variables|/Game/D_ufo/ufo.ufo_C|GetHealth _asufo) 0.1)))

(event OnComponentBeginOverlap(d12)
  (params (OverlappedComponent :type Primitive%20Component%20Object%20Reference) (OtherActor :type Actor%20Object%20Reference) (OtherComp :type Primitive%20Component%20Object%20Reference) (OtherBodyIndex :type Integer) (bFromSweep :type Boolean) (SweepResult :type Hit%20Result%20Structure%20%28by%20ref%29))
  (bind _asufo (Utilities|Casting|CastToufo OtherActor))
  (Variables|/Game/D_ufo/ufo.ufo_C|SetHealth _asufo (- (Variables|/Game/D_ufo/ufo.ufo_C|GetHealth _asufo) 0.1)))

(event OnComponentBeginOverlap(d13)
  (params (OverlappedComponent :type Primitive%20Component%20Object%20Reference) (OtherActor :type Actor%20Object%20Reference) (OtherComp :type Primitive%20Component%20Object%20Reference) (OtherBodyIndex :type Integer) (bFromSweep :type Boolean) (SweepResult :type Hit%20Result%20Structure%20%28by%20ref%29))
  (bind _asufo (Utilities|Casting|CastToufo OtherActor))
  (Variables|/Game/D_ufo/ufo.ufo_C|SetHealth _asufo (- (Variables|/Game/D_ufo/ufo.ufo_C|GetHealth _asufo) 0.1)))

(event OnComponentBeginOverlap(d14)
  (params (OverlappedComponent :type Primitive%20Component%20Object%20Reference) (OtherActor :type Actor%20Object%20Reference) (OtherComp :type Primitive%20Component%20Object%20Reference) (OtherBodyIndex :type Integer) (bFromSweep :type Boolean) (SweepResult :type Hit%20Result%20Structure%20%28by%20ref%29))
  (bind _asufo (Utilities|Casting|CastToufo OtherActor))
  (Variables|/Game/D_ufo/ufo.ufo_C|SetHealth _asufo (- (Variables|/Game/D_ufo/ufo.ufo_C|GetHealth _asufo) 0.1)))

(event OnComponentBeginOverlap(d11)
  (params (OverlappedComponent :type Primitive%20Component%20Object%20Reference) (OtherActor :type Actor%20Object%20Reference) (OtherComp :type Primitive%20Component%20Object%20Reference) (OtherBodyIndex :type Integer) (bFromSweep :type Boolean) (SweepResult :type Hit%20Result%20Structure%20%28by%20ref%29))
  (bind _asufo (Utilities|Casting|CastToufo OtherActor))
  (Variables|/Game/D_ufo/ufo.ufo_C|SetHealth _asufo (- (Variables|/Game/D_ufo/ufo.ufo_C|GetHealth _asufo) 0.1)))

(event OnComponentBeginOverlap(d1)
  (params (OverlappedComponent :type Primitive%20Component%20Object%20Reference) (OtherActor :type Actor%20Object%20Reference) (OtherComp :type Primitive%20Component%20Object%20Reference) (OtherBodyIndex :type Integer) (bFromSweep :type Boolean) (SweepResult :type Hit%20Result%20Structure%20%28by%20ref%29))
  (bind _asufo (Utilities|Casting|CastToufo OtherActor))
  (Variables|/Game/D_ufo/ufo.ufo_C|SetHealth _asufo (- (Variables|/Game/D_ufo/ufo.ufo_C|GetHealth _asufo) 0.1)))

(event EventBeginPlay
  (bind _mutiattack2 (Variables|Default|GetMutiAttack2))
  (Utilities|FlowControl|Delay (Variables|Default|Gettime_exist))
  (Effects|SpawnEmitteratLocation "/Game/EnemyMaterialAndParticle/P_ProjectileLob_Explo_Ice_02.P_ProjectileLob_Explo_Ice_02" (Transformation|GetWorldLocation _mutiattack2) (Transformation|GetWorldRotation _mutiattack2))
  (Actor|DestroyActor))

(fn ConstructionScript)