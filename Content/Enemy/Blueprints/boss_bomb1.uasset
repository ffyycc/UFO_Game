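; A timed boss bomb that explodes after a set lifetime and is meant to damage the ufo.
; After the TimeExist delay it sets Explode, spawns a scaled-up explosion emitter at its sphere and destroys itself immediately.
; Range_bomb begin-overlap subtracts a small fixed amount of ufo Health only while Explode is set, so a ufo already inside gets no explicit damage check at detonation.
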(event OnComponentBeginOverlap(range_bomb)
  (params (OverlappedComponent :type Primitive%20Component%20Object%20Reference) (OtherActor :type Actor%20Object%20Reference) (OtherComp :type Primitive%20Component%20Object%20Reference) (OtherBodyIndex :type Integer) (bFromSweep :type Boolean) (SweepResult :type Hit%20Result%20Structure%20%28by%20ref%29))
  (bind _asufo (Utilities|Casting|CastToufo OtherActor))
  (if (Variables|Default|Getexplode)
    (Variables|/Game/D_ufo/ufo.ufo_C|SetHealth _asufo (- (Variables|/Game/D_ufo/ufo.ufo_C|GetHealth _asufo) 0.2))))

(event EventBeginPlay
  (bind _sphere (Variables|Default|GetSphere))
  ;[1 1 1] bomb damage
  (Utilities|FlowControl|Delay (Variables|Default|Gettime_exist))
  (Variables|Default|Setexplode true)
  (Effects|SpawnEmitteratLocation "/Game/EnemyMaterialAndParticle/P_BomberExplode.P_BomberExplode" (Transformation|GetWorldLocation _sphere) (Transformation|GetWorldRotation _sphere) "10.000000,10.000000,10.000000")
  (Actor|DestroyActor))

(fn ConstructionScript)